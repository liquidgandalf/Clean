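; Pickup briefcase that collects special items and, once flagged full, acts as a key for interactable objects with a matching lock code.
; Tick detects grab changes: grabbing swaps to the closed lid and snaps overlapping code-2 items into free sockets among four slots, lighting up when full.
; Releasing opens the lid, detaches items with physics and clears the slots.
; Actor overlap while flagged full unlocks and triggers the matching object.
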(event `self.ReceiveTick`
  (params (DeltaSeconds :type "Float (single-precision)"))
  (bind _lid2 (`self.Lid2`))
  (bind _lid2_2 (`self.Lid2`))
  (bind _slots (`self.Slots`))
  (bind _caserep (`self.CaseRep`))
  (bind _slots_2 (`self.Slots`))
  ;[1 1 1] Test to see if Grabbed Status has Changed
  (if (not (== (`self.LastGrab`) (`self.BP_PickupCudeIsGrabbed?`)))
    (set `self.LastGrab` (`self.BP_PickupCudeIsGrabbed?`))
    (if (`self.BP_PickupCudeIsGrabbed?`)
      ;[1 1 1] Change Viewport to Is Grabbed - Close The Case
      (`SceneComponent.SetVisibility` (`self.Lid1`) false false)
      (`SceneComponent.SetVisibility` _lid2 true false)
      (`PrimitiveComponent.SetCollisionEnabled` _lid2 "PhysicsOnly")
      (`PrimitiveComponent.SetCollisionEnabled` (`self.Lid1`) "NoCollision")
      ;[1 1 1] Attach Each Item to a Free Slot
      (for _array_element (`PrimitiveComponent.GetOverlappingActors` (`self.Box`) "/Game/Assets_Dereks/DL_Blueprints/BP_SpecialItems_Pickup.BP_SpecialItems_Pickup_C")
        (bind _asbp_special_items_pickup (cast `/Game/Assets_Dereks/DL_Blueprints/BP_SpecialItems_Pickup` _array_element))
        (if (== (`/Game/Assets_Dereks/DL_Blueprints/BP_SpecialItems_Pickup.BP_PickupCudeItemCode` _asbp_special_items_pickup) 2)
          (for (_array_element_2 _array_index) _slots
            (if (not _array_element_2)
              (break)))
          (`KismetArrayLibrary.Array_Set` _slots _array_index true)
          (switch `int` _array_index
            (:`0`
              (`self.K2_AttachToComponent` _array_element _caserep "Slot1" "SnapToTarget" "SnapToTarget" "KeepWorld" true)
              (`KismetArrayLibrary.Array_Set` _slots_2 0 true))
            (:`1`
              (`self.K2_AttachToComponent` _array_element _caserep "Slot2" "SnapToTarget" "SnapToTarget" "KeepWorld" true)
              (`KismetArrayLibrary.Array_Set` _slots_2 1 true))
            (:`2`
              (`self.K2_AttachToComponent` _array_element _caserep "Slot3" "SnapToTarget" "SnapToTarget" "KeepWorld" true)
              (`KismetArrayLibrary.Array_Set` _slots_2 2 true))
            (:`3`
              (`self.K2_AttachToComponent` _array_element _caserep "Slot4" "SnapToTarget" "SnapToTarget" "KeepWorld" true)
              (`KismetArrayLibrary.Array_Set` _slots_2 3 true)))
          (set `self.GotItems` true)
          ;[1 1 1] IsCaseFull? Turn light on
          (for _array_element_3 (`self.Slots`)
            (if _array_element_3
              (set `self.IsCaseFull` true)
              (else
                (set `self.IsCaseFull` false)
                (break))))
          (if (`self.IsCaseFull`)
            (`LightComponent.SetIntensity` (`self.PointLight1`) 5000.0)
            (else
              (`LightComponent.SetIntensity` (`self.PointLight1`) 0.0)))))
      (else
        ;[1 1 1] Change Viewport Is Not Grabbed
        (`SceneComponent.SetVisibility` (`self.Lid1`) true false)
        (`SceneComponent.SetVisibility` _lid2_2 false false)
        (`PrimitiveComponent.SetCollisionEnabled` _lid2_2 "NoCollision")
        (`PrimitiveComponent.SetCollisionEnabled` (`self.Lid1`) "NoCollision")
        ;[1 1 1] Release Let Go of the Items - No Force
        (if (`self.GotItems`)
          (for _array_element_4 (`PrimitiveComponent.GetOverlappingActors` (`self.Box`) "/Game/Assets_Dereks/DL_Blueprints/BP_SpecialItems_Pickup.BP_SpecialItems_Pickup_C")
            (bind _asbp_special_items_pickup_2 (cast `/Game/Assets_Dereks/DL_Blueprints/BP_SpecialItems_Pickup` _array_element_4))
            (`self.K2_DetachFromActor` _asbp_special_items_pickup_2 "KeepWorld" "KeepWorld" "KeepWorld")
            (`PrimitiveComponent.SetSimulatePhysics` (`StaticMeshActor.StaticMeshComponent` _asbp_special_items_pickup_2) true)
            (`self.OutputSlotStatus`)
            (`LightComponent.SetIntensity` (`self.PointLight1`) 0.0))
          (set `self.Slots` (`self.EmptySlots`)))))))

(event `self.ReceiveActorBeginOverlap`
  (params (OtherActor :type "Actor Object Reference"))
  (if (`self.IsCaseFull`)
    (if (== (`GameplayStatics.GetObjectClass` OtherActor) "/Game/Assets_Dereks/DL_Blueprints/BP_Interact_Object.BP_Interact_Object_C")
      (bind _asbp_interact_object (cast `/Game/Assets_Dereks/DL_Blueprints/BP_Interact_Object` OtherActor))
      (if (== (`/Game/Assets_Dereks/DL_Blueprints/BP_Interact_Object.DoorLockCode` _asbp_interact_object) (`self.DoorUnLockCode`))
        (`/Game/Assets_Dereks/DL_Blueprints/BP_Interact_Object.Unlock_Door` _asbp_interact_object)
        (`/Game/Assets_Dereks/DL_Blueprints/BP_Interact_Object.Interact_With_Object` _asbp_interact_object)))))

(fn `OutputSlotStatus`
  (for (_array_element _array_index) (`self.Slots`)
    (`KismetSystemLibrary.PrintText` (`|FormatText` "*Slot {0} Is {1}" _array_index (`KismetTextLibrary.Conv_BoolToText` _array_element)))))

(fn `UserConstructionScript`
  (`parent.UserConstructionScript`))