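; Solid interactable door with a point light whose colour shows whether it is locked or unlocked.
; Construction extends the parent script, applying an optional SolidDoorMesh to DefaultMesh.
; While the door moves, Tick snaps the secondary SolidDoorBit to DefaultMesh's transform and refreshes the light.
; When stationary, it polls IsLocked and recolours on change; showing the status from BeginPlay is optional.
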(event `self.ReceiveBeginPlay`
  (set `self.LightLast` (`self.IsLocked?`))
  (if (`self.ShowLockStatusFromStart`)
    (`self.SetColour`)))

(event `self.ReceiveTick`
  (params (DeltaSeconds :type "Float (single-precision)"))
  (bind _soliddoorbit (`self.SolidDoorBit`))
  (bind _islocked_ (`self.IsLocked?`))
  (bind _returnvalue (`SceneComponent.K2_GetComponentToWorld` (`self.DefaultMesh`)))
  ;[1 1 1] Move the 2ndary door to main door if moving
  (if (`self.IsMoving`)
    (if (not (== _returnvalue (`SceneComponent.K2_GetComponentToWorld` _soliddoorbit)))
      (`SceneComponent.K2_SetWorldTransform` _soliddoorbit _returnvalue false false)
      (`self.SetColour`))
    (else
      ;[1 1 1] Change Colour?
      (if (not (== (`self.LightLast`) _islocked_))
        (set `self.LightLast` _islocked_)
        (`self.SetColour`)))))

(fn `SetColour`
  (bind _pointlight (`self.PointLight`))
  (if (`self.IsLocked?`)
    (`LightComponent.SetLightColor` _pointlight (`self.ColourLocked`) true)
    (else
      (`LightComponent.SetLightColor` _pointlight (`self.ColourUnlocked`) true))))

(fn `UserConstructionScript`
  (bind _soliddoormesh (`self.SolidDoorMesh`))
  (`parent.UserConstructionScript`)
  (if (!= _soliddoormesh null)
    (`StaticMeshComponent.SetStaticMesh` (`self.DefaultMesh`) _soliddoormesh)))