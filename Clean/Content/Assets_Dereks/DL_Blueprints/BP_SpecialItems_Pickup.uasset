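; BP_SpecialItems_Pickup is a pickup item that motion controllers grab and drop, with an optional point light.
; Pickup disables physics and attaches the actor to the given component's Handle socket; Drop reverses both.
; BeginPlay configures the light when enabled, and ToggleLight flips its visibility.
; Disconnected key logic would match item codes against doors and interactables to unlock or trigger them, but the overlap event does nothing.
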(event `self.ReceiveBeginPlay`
  (bind _pointlight (`self.PointLight`))
  ;[1 1 1] Begin Play Set up the Light
  (if (`self.BP_PickUpCubeLightOn`)
    (`LightComponent.SetIntensity` _pointlight (`self.StartIntensity`))
    (`LightComponent.SetLightColor` _pointlight (`self.BP_PickupCubeLightColour`) true)
    (`SceneComponent.SetVisibility` _pointlight true false)
    (set `self.BP_PickUpCubeLightOn` true)))

(event `/Game/VirtualRealityBP/Blueprints/PickupActorInterface.Pickup`
  (params (AttachTo :type "SceneComponent Object Reference"))
  ;[1 1 1] Pickup Drop Not My Bp
  (set `self.BP_PickupCudeIsGrabbed?` true)
  (`PrimitiveComponent.SetSimulatePhysics` (`self.StaticMeshComponent`) false)
  (`SceneComponent.K2_AttachToComponent` (`self.K2_GetRootComponent`) AttachTo "Handle" "KeepWorld" "KeepWorld" "KeepWorld" false))

(event `/Game/VirtualRealityBP/Blueprints/PickupActorInterface.Drop`
  ;[1 1 1] Pickup Drop Not My Bp
  (set `self.BP_PickupCudeIsGrabbed?` false)
  (`PrimitiveComponent.SetSimulatePhysics` (`self.StaticMeshComponent`) true)
  (`self.K2_DetachFromActor` "KeepWorld" "KeepWorld" "KeepWorld"))

(event `self.ReceiveActorBeginOverlap`
  (params (OtherActor :type "Actor Object Reference")))

(fn `ToggleLight`
  (if (`self.BP_PickUpCubeLightOn`)
    (set `self.BP_PickUpCubeLightOn` false)
    (else
      (set `self.BP_PickUpCubeLightOn` true)))
  (`SceneComponent.SetVisibility` (`self.PointLight`) (`self.BP_PickUpCubeLightOn`) false))

(fn `UserConstructionScript`)