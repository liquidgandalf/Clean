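; BP_ItemChucker is an actor that spawns a set number of physics-driven BP_Racket items when play begins.
; A BeginPlay loop spawns them all at once at its StaticMesh's transform, replacing the pitch with a random value.
; Each racket gets physics simulation and a fixed angular velocity, so it starts out spinning.
; An unconnected calculation for stacking spawn height by count is left unused.
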(event `self.ReceiveBeginPlay`
  (bind _numberspawned (`self.NumberSpawned`))
  (bind _returnvalue (`SceneComponent.K2_GetComponentToWorld` (`self.StaticMesh`)))
  ;[1 1 1] Spawn a Set Number of Items
  (`KismetSystemLibrary.PrintText` "*Start Of Spawn")
  (while (> (`self.NumberToSpawn`) _numberspawned)
    (bind _output_get (set `self.NumberSpawned` (+ _numberspawned 1)))
    (bind _returnvalue_2 (`|SpawnActorFromClass` "/Game/Z_JUNK/BP_Racket.BP_Racket_C" (`KismetMathLibrary.MakeTransform` (`KismetMathLibrary.MakeVector` (.x (.location _returnvalue)) (.y (.location _returnvalue)) (.z (.location _returnvalue))) (`KismetMathLibrary.MakeRotator` (.roll (.rotation _returnvalue)) (`KismetMathLibrary.Conv_IntToDouble` (`KismetMathLibrary.RandomInteger` 300)) (.yaw (.rotation _returnvalue))) (.scale _returnvalue)) "Undefined" "OverrideRootScale"))
    (`PrimitiveComponent.SetSimulatePhysics` (`/Game/Z_JUNK/BP_Racket.StaticMesh` _returnvalue_2) true)
    (`PrimitiveComponent.SetPhysicsAngularVelocity` (`/Game/Z_JUNK/BP_Racket.StaticMesh` _returnvalue_2) (25.0 200.0 0.0) false "None")))

(fn `UserConstructionScript`)