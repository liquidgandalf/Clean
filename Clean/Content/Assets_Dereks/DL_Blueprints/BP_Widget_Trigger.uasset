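; Trigger actor that shows one of four menus on overlap: player name keyboard, server name keyboard, host menu or join menu.
; On begin overlap, WidgetNumber selects the widget to create, then a shared AddToViewport call targets all four references and the mouse cursor appears.
; On end overlap, it hides the cursor and removes the selected widget.
; Neither event filters the overlapping actor, and both use player controller 0.
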(event `self.ReceiveActorBeginOverlap`
  (params (OtherActor :type "Actor Object Reference"))
  ;[1 1 1] OpenWidgetOnScreen
  (switch `int` (`self.WidgetNumber`)
    (:`0`
      (bind _returnvalue (`|CreateWidget` "/Game/Assets_Dereks/DL_Maps_Specials/VR_MP_MainStart/Widgets/VR_KB_PlayerName.VR_KB_PlayerName_C" null "Header Text"))
      (bind _output_get (set `self.PlayerNameWG` _returnvalue)))
    (:`1`
      (bind _returnvalue_2 (`|CreateWidget` "/Game/Assets_Dereks/DL_Maps_Specials/VR_MP_MainStart/Widgets/VR_KB_ServerName.VR_KB_ServerName_C" null "Header Text"))
      (bind _output_get_2 (set `self.ServerNameWG` _returnvalue_2)))
    (:`2`
      (bind _returnvalue_3 (`|CreateWidget` "/Game/Assets_Dereks/DL_Maps_Specials/VR_MP_MainStart/Widgets/VR_HostMenu.VR_HostMenu_C"))
      (bind _output_get_3 (set `self.HostSettingsWG` _returnvalue_3)))
    (:`3`
      (bind _returnvalue_4 (`|CreateWidget` "/Game/Assets_Dereks/DL_Maps_Specials/VR_MP_MainStart/Widgets/VT_Join_Menu.VT_Join_Menu_C"))
      (bind _output_get_4 (set `self.JoinSettingsWG` _returnvalue_4))))
  (`UserWidget.AddToViewport` _output_get 0)
  (`UserWidget.AddToViewport` _output_get_2 0)
  (`UserWidget.AddToViewport` _output_get_3 0)
  (`UserWidget.AddToViewport` _output_get_4 0)
  (set `PlayerController.bShowMouseCursor` true (`GameplayStatics.GetPlayerController` 0)))

(event `self.ReceiveActorEndOverlap`
  (params (OtherActor :type "Actor Object Reference"))
  (set `PlayerController.bShowMouseCursor` false (`GameplayStatics.GetPlayerController` 0))
  (switch `int` (`self.WidgetNumber`)
    (:`0`
      (`Widget.RemoveFromParent` (`self.PlayerNameWG`)))
    (:`1`
      (`Widget.RemoveFromParent` (`self.ServerNameWG`)))
    (:`2`
      (`Widget.RemoveFromParent` (`self.HostSettingsWG`)))
    (:`3`
      (`Widget.RemoveFromParent` (`self.JoinSettingsWG`)))))

(fn `UserConstructionScript`)